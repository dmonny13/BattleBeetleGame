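; Scorpion enemy that chases and attacks the side-scroller player character, and opens the Congrats level when killed.
; Pawn sensing starts an AI move toward the player, then plays the fight montage and applies damage on arrival.
; Tick re-issues the chase using the last sensed pawn and checks health, which AnyDamage lowers.
; A separate DamagePlayer event also applies damage to a Player reference.
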(event `self.ReceiveAnyDamage`
  (params (Damage :type "Float (single-precision)") (DamageType :type "DamageType Object Reference") (InstigatedBy :type "Controller Object Reference") (DamageCauser :type "Actor Object Reference"))
  (set `self.ScpHealth` (- (`self.ScpHealth`) Damage)))

(event `self.ReceiveBeginPlay`
  (set `self.ScpHealth` 5.0))

(event `self.ReceiveTick`
  (params (DeltaSeconds :type "Float (single-precision)"))
  (bind _asside_scroller_character (cast `/Game/SideScrollerBP/Blueprints/SideScrollerCharacter` (stale `self.PawnSensing.OnSeePawn` Pawn)))
  (if (<= (`self.ScpHealth`) 0.0)
    (`self.K2_DestroyActor`)
    (`GameplayStatics.OpenLevel` "Congrats")
    (else
      (`|AIMoveTo` self (0.0 0.0 0.0) _asside_scroller_character 10.0 true))))

(event `self.PawnSensing.OnSeePawn`
  (params (Pawn :type "Pawn Object Reference"))
  (bind _asside_scroller_character (cast `/Game/SideScrollerBP/Blueprints/SideScrollerCharacter` Pawn))
  (`|AIMoveTo` self (0.0 0.0 0.0) _asside_scroller_character 10.0 true
    (:`OnSuccess`
      (`AnimInstance.Montage_Play` (`SkeletalMeshComponent.GetAnimInstance` (`self.Mesh`)) "/Game/Scorpion/Animations/ScorpionFight.ScorpionFight" 0.75 "MontageLength" 0.0 false)
      (`GameplayStatics.ApplyDamage` _asside_scroller_character (`self.Damage`) null self)
      (`KismetSystemLibrary.Delay` 1.0))))

(event `Damage Player`
  (`GameplayStatics.ApplyDamage` (`self.Player`) (`self.Damage`) null self))

(fn `UserConstructionScript`)